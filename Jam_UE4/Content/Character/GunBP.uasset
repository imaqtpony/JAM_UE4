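; Gun Blueprint that fires bullets for as long as the Shoot input is held.
; It enables player input on BeginPlay and feeds Shoot press and release into a Hold Input macro.
; The macro uses a Gate and Retriggerable Delay loop to fire at once, then repeat every TimeBetweenBullets until released.
; Each shot spawns a BulletBP at BulletSpawnPoint with a short life span.
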(event `self.ReceiveBeginPlay`
  ;[0.2604 0.2604 0.2604] Enable Inputs
  (`self.EnableInput` (`GameplayStatics.GetPlayerController` 0)))

(event `InputAction|Shoot`
  (params (Key :type "Key Structure"))
  ;[0.1305 0.08439 0.2865] Instantiate Bullet
  (:`Pressed`
    (`|ExecutionSequence`
      (:`then_0`
        (goto _label :!via `Open`))
      (:`then_1`
        (`/Engine/EditorBlueprintResources/StandardMacros.Gate` true :!label _label
          (:`Exit`
            (`|ExecutionSequence`
              (:`then_0`
                (bind _returnvalue (`|SpawnActorFromClass` "/Game/Character/BulletBP.BulletBP_C" (`SceneComponent.K2_GetComponentToWorld` (`self.BulletSpawnPoint`)) "AlwaysSpawn" "OverrideRootScale" null null))
                (bind _output_get (set `self.Bullet` _returnvalue))
                (`self.SetLifeSpan` _output_get 3.0))
              (:`then_1`
                (`KismetSystemLibrary.RetriggerableDelay` (`self.TimeBetweenBullets`))
                (goto _label))))))))
  (:`Released`
    (goto _label :!via `Close`)))

(fn `UserConstructionScript`)