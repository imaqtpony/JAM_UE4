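; Player character Blueprint that handles axis-driven movement, facing and an impulse dash.
; Movement inputs push along fixed world forward and right axes unless DisableMovement is set.
; Dash applies a velocity-change impulse along an input-axis vector scaled by DashForce, using a DoOnce that resets after a delay on release to prevent spam.
; Tick turns the actor toward a non-zero input-axis vector, stored as Orientation.
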(event `InputAxis|MoveHorizontal`
  (params (AxisValue :type "Float (single-precision)"))
  ;[0.07235 0.09565 0.3021] Movement
  (if (not (`self.DisableMovement`))
    (`self.AddMovementInput` (`KismetMathLibrary.GetRightVector` (struct)) AxisValue)))

(event `InputAction|Dash`
  (params (Key :type "Key Structure"))
  ;[0.3542 0.2203 0.1593] Dash
  ;;[1 1 1] Get the input and add a delay to prevent spam
  (:`Pressed`
    (`/Engine/EditorBlueprintResources/StandardMacros.DoOnce` false :!label _label
      (:`Completed`
        (`CharacterMovementComponent.AddImpulse` (`self.CharacterMovement`) (* (`KismetMathLibrary.MakeVector` (stale `InputAxis|MoveVertical` AxisValue) (stale `InputAxis|MoveHorizontal` AxisValue)) (`self.DashForce`)) true))))
  (:`Released`
    (`KismetSystemLibrary.Delay` (`self.DelayBetweenDash`))
    (goto _label :!via `Reset`)))

(event `InputAxis|MoveVertical`
  (params (AxisValue :type "Float (single-precision)"))
  ;[0.07235 0.09565 0.3021] Movement
  (if (not (`self.DisableMovement`))
    (`self.AddMovementInput` (`KismetMathLibrary.GetForwardVector` (struct)) AxisValue)))

(event `self.ReceiveTick`
  (params (DeltaSeconds :type "Float (single-precision)"))
  ;[0.3253 0.5885 0.2648] Rotate
  (bind _returnvalue (`KismetMathLibrary.MakeVector` (stale `InputAxis|AimVertical` AxisValue) (stale `InputAxis|AimHorizontal` AxisValue)))
  (bind _output_get (set `self.Orientation` _returnvalue))
  (if (not (`KismetMathLibrary.Vector_IsZero` _returnvalue))
    (`self.K2_SetActorRotation` (`KismetMathLibrary.MakeRotFromX` (`KismetMathLibrary.Normal` _output_get)))))

(event `InputAxis|AimVertical`
  (params (AxisValue :type "Float (single-precision)"))
  ;[0.3253 0.5885 0.2648] Rotate
)

(event `InputAxis|AimHorizontal`
  (params (AxisValue :type "Float (single-precision)"))
  ;[0.3253 0.5885 0.2648] Rotate
)

(fn `UserConstructionScript`)